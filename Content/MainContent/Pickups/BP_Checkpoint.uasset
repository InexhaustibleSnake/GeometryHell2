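; BP_Checkpoint is a one-shot checkpoint pickup that saves the player's progress when the player character overlaps it.
; It loads the save data if the game instance's slot already exists, or otherwise creates a new BP_PlayerData object.
; It stores its own transform, the current level name and the game instance's core count, saves the data, then destroys itself.
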(event `self.ReceiveActorBeginOverlap`
  (params (OtherActor :type "Actor Object Reference"))
  (if (== OtherActor (`GameplayStatics.GetPlayerCharacter` 0))
    (bind _returnvalue (`GameplayStatics.DoesSaveGameExist` (`/Game/MainContent/Logic/BP_MainGameInstance.SaveSlot` (`/Game/MainContent/Logic/BFL_Main.GetMainGameInstance`))))
    (if _returnvalue
      (bind _asbp_player_data (`/Game/MainContent/Logic/BFL_Main.LoadSaveData`))
      (set `self.SaveData` _asbp_player_data)
      (else
        (bind _returnvalue_2 (`GameplayStatics.CreateSaveGameObject` "/Game/MainContent/Logic/Saves/BP_PlayerData.BP_PlayerData_C"))
        (set `self.SaveData` _returnvalue_2)))
    (bind _returnvalue_3 (`GameplayStatics.GetCurrentLevelName` true))
    (set `/Game/MainContent/Logic/Saves/BP_PlayerData.LevelAndTransformData` (make `/Game/MainContent/Logic/Saves/SBP_LevelAndTransform` (`self.GetTransform`) _returnvalue_3) (`self.SaveData`))
    (set `/Game/MainContent/Logic/Saves/BP_PlayerData.CoresAmount` (`MainGameInstance.GetCores` (`/Game/MainContent/Logic/BFL_Main.GetMainGameInstance`)) (`self.SaveData`))
    (`/Game/MainContent/Logic/BFL_Main.SaveGameData` (`self.SaveData`))
    (`self.K2_DestroyActor`)))

(fn `UserConstructionScript`)