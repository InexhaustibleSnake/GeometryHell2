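; BP_BaseEnemy is a base enemy Blueprint that gives visual hit feedback on its cannon mesh.
; BeginPlay applies the default material and binds a handler to the actor's any-damage event.
; On damage, the handler swaps to the hurt material and restores the default after a brief delay, producing a flash.
; The graph contains no health or death logic.
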(event `self.ReceiveBeginPlay`
  (`PrimitiveComponent.SetMaterial` (`self.CannonMesh`) 0 (`self.DefaultMaterial`))
  (add `Actor.OnTakeAnyDamage` (delegate `OnTakeAnyDamage_Event_0`)))

(event `OnTakeAnyDamage_Event_0`
  (params (DamagedActor :type "Actor Object Reference") (Damage :type "Float (double-precision)") (DamageType :type "DamageType Object Reference") (InstigatedBy :type "Controller Object Reference") (DamageCauser :type "Actor Object Reference"))
  (`PrimitiveComponent.SetMaterial` (`self.CannonMesh`) 0 (`self.HurtMaterial`))
  (`KismetSystemLibrary.Delay` 0.1)
  (`PrimitiveComponent.SetMaterial` (`self.CannonMesh`) 0 (`self.DefaultMaterial`)))

(fn `UserConstructionScript`)