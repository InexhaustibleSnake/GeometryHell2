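; BP_IllusionerEnemy is an enemy that hijacks the player's view, forcing the control rotation to face its mesh every tick.
; The look-at runs from the player controller's location, keeping its roll, with no range or state check.
; Taking damage briefly swaps the cannon mesh to a hurt material as a flash.
; On death it increments the level kill count, adds its core reward to the level total and saves the game.
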(event `self.ReceiveTick`
  (params (DeltaSeconds :type "Float (single-precision)"))
  (bind _returnvalue_roll (`KismetMathLibrary.BreakRotator` (`self.K2_GetActorRotation` (`GameplayStatics.GetPlayerController` 0))))
  (bind (_returnvalue_roll_2 _returnvalue_pitch _returnvalue_yaw) (`KismetMathLibrary.BreakRotator` (`KismetMathLibrary.FindLookAtRotation` (`self.K2_GetActorLocation` (`GameplayStatics.GetPlayerController` 0)) (`SceneComponent.K2_GetComponentLocation` (`self.Mesh`)))))
  (`Controller.SetControlRotation` (`GameplayStatics.GetPlayerController` 0) (`KismetMathLibrary.MakeRotator` _returnvalue_roll _returnvalue_pitch _returnvalue_yaw)))

(event `self.ReceiveBeginPlay`
  (`PrimitiveComponent.SetMaterial` (`self.CannonMesh`) 0 (`self.DefaultMaterial`))
  (add `self.OnTakeAnyDamage` (delegate `OnTakeAnyDamage_Event_0`))
  (add `self.OnDeath` (delegate `OnDeath_Event_0`)))

(event `OnTakeAnyDamage_Event_0` :!signature `self.OnTakeAnyDamage`
  (params (DamagedActor :type "Actor Object Reference") (Damage :type "Float (double-precision)") (DamageType :type "DamageType Object Reference") (InstigatedBy :type "Controller Object Reference") (DamageCauser :type "Actor Object Reference"))
  (`PrimitiveComponent.SetMaterial` (`self.CannonMesh`) 0 (`self.HurtMaterial`))
  (`KismetSystemLibrary.Delay` 0.1)
  (`PrimitiveComponent.SetMaterial` (`self.CannonMesh`) 0 (`self.DefaultMaterial`)))

(event `OnDeath_Event_0`
  (bind (_currentleveldata_coresobtainedinlevel _currentleveldata_enemieskilledinlevel) (break `/Game/MainContent/Logic/Saves/SBP_CurrentLevelData` (`/Game/MainContent/Logic/Saves/BP_PlayerData.CurrentLevelData` (`self.SaveData`))))
  (bind _currentleveldata_coresobtainedinlevel_2 (break `/Game/MainContent/Logic/Saves/SBP_CurrentLevelData` (`/Game/MainContent/Logic/Saves/BP_PlayerData.CurrentLevelData` (`self.SaveData`))))
  (bind _asbp_player_data (`/Game/MainContent/Logic/BFL_Main.LoadSaveData`))
  (set `self.SaveData` _asbp_player_data)
  (bind _result (`/Engine/EditorBlueprintResources/StandardMacros.IncrementInt` _currentleveldata_enemieskilledinlevel)
    (:`  `
      (set `/Game/MainContent/Logic/Saves/BP_PlayerData.CurrentLevelData` (make `/Game/MainContent/Logic/Saves/SBP_CurrentLevelData` (+ _currentleveldata_coresobtainedinlevel_2 (`self.CoresForKill`)) _result) (`self.SaveData`))
      (`/Game/MainContent/Logic/BFL_Main.SaveGameData` (`self.SaveData`)))))

(fn `UserConstructionScript`)