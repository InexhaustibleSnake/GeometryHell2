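; BP_BossBase is a base Blueprint for boss enemies, adding a boss health bar and kill rewards on top of its parent's behavior.
; On BeginPlay it creates the health bar widget, adds it to the viewport and binds to the OnDeath event.
; On death it removes the bar, loads save data, increments the level's kill count, adds the cores for the kill and saves.
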(event `self.ReceiveBeginPlay`
  (`parent.ReceiveBeginPlay`)
  (bind _returnvalue (`|CreateWidget` (`self.Class`)))
  (`/Engine/EditorBlueprintResources/StandardMacros.IsValid` _returnvalue
    (:`Is Valid`
      (bind _output_get (set `self.BossHealthBar` _returnvalue))
      (`UserWidget.AddToViewport` _output_get 0)
      (add `self.OnDeath` (delegate `OnDeath_Event_0`)))))

(event `OnDeath_Event_0`
  (bind (_currentleveldata_coresobtainedinlevel _currentleveldata_enemieskilledinlevel) (break `/Game/MainContent/Logic/Saves/SBP_CurrentLevelData` (`/Game/MainContent/Logic/Saves/BP_PlayerData.CurrentLevelData` (`self.SaveData`))))
  (bind _currentleveldata_coresobtainedinlevel_2 (break `/Game/MainContent/Logic/Saves/SBP_CurrentLevelData` (`/Game/MainContent/Logic/Saves/BP_PlayerData.CurrentLevelData` (`self.SaveData`))))
  (`Widget.RemoveFromParent` (`self.BossHealthBar`))
  (bind _asbp_player_data (`/Game/MainContent/Logic/BFL_Main.LoadSaveData`))
  (set `self.SaveData` _asbp_player_data)
  (bind _result (`/Engine/EditorBlueprintResources/StandardMacros.IncrementInt` _currentleveldata_enemieskilledinlevel)
    (:`  `
      (set `/Game/MainContent/Logic/Saves/BP_PlayerData.CurrentLevelData` (make `/Game/MainContent/Logic/Saves/SBP_CurrentLevelData` (+ _currentleveldata_coresobtainedinlevel_2 (`self.CoresForKill`)) _result) (`self.SaveData`))
      (`/Game/MainContent/Logic/BFL_Main.SaveGameData` (`self.SaveData`)))))

(fn `UserConstructionScript`
  (`parent.UserConstructionScript`))