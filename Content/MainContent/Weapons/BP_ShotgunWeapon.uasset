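; Shotgun weapon Blueprint that syncs its tuning values with the WeaponParameters save slot on BeginPlay.
; If the save exists, it loads it and overrides projectile damage, fire rate and projectile count from the stored shotgun parameters.
; Otherwise it creates a new BP_WeaponParametersSave seeded with its own current values and writes it to the slot.
; No firing logic is defined in these graphs.
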(event `self.ReceiveBeginPlay`
  (bind _returnvalue (`GameplayStatics.DoesSaveGameExist` "WeaponParameters"))
  (if _returnvalue
    (bind _returnvalue_2 (`GameplayStatics.LoadGameFromSlot` "WeaponParameters"))
    (bind _asbp_weapon_parameters_save (cast `/Game/MainContent/Logic/Saves/BP_WeaponParametersSave` _returnvalue_2))
    (bind _output_get (set `self.WeaponParametersSave` _asbp_weapon_parameters_save))
    (bind (_shotgundamage _shotgunfirerate _shotgunnumofprojectiles) (`/Game/MainContent/Logic/Saves/BP_WeaponParametersSave.GetShotgunParams` _output_get))
    (set `self.ProjectileDamage` _shotgundamage)
    (set `self.FireRate` _shotgunfirerate)
    (set `self.NumOfProjectiles` _shotgunnumofprojectiles)
    (else
      (bind _returnvalue_3 (`GameplayStatics.CreateSaveGameObject` "/Game/MainContent/Logic/Saves/BP_WeaponParametersSave.BP_WeaponParametersSave_C"))
      (`/Game/MainContent/Logic/Saves/BP_WeaponParametersSave.SetShotgunParams` _returnvalue_3 (`self.ProjectileDamage`) (`self.FireRate`) (`self.NumOfProjectiles`))
      (`GameplayStatics.SaveGameToSlot` _returnvalue_3 "WeaponParameters"))))

(fn `UserConstructionScript`)