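; Sniper rifle projectile that homes in on nearby BaseEnemy actors.
; On BeginPlay it copies HomingPower from the first BP_SniperRifleWeapon in the world into its movement component's homing acceleration.
; It then re-runs FindEnemy every 0.2 seconds to set the homing target.
; FindEnemy scans all enemies against a stored ClosestDistance that is never reset, so the target changes only when an enemy beats that record.
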(event `self.ReceiveBeginPlay`
  (bind _outactors (`GameplayStatics.GetAllActorsOfClass` "/Game/MainContent/Weapons/BP_SniperRifleWeapon.BP_SniperRifleWeapon_C"))
  (bind _output_get (set `self.HomingPower` (`/Game/MainContent/Weapons/BP_SniperRifleWeapon.HomingPower` (`|GetArrayItem` _outactors))))
  (set `ProjectileMovementComponent.HomingAccelerationMagnitude` _output_get (`self.ProjectileMovementComponent`))
  (`self.GoToTarget` :!label _label)
  (`KismetSystemLibrary.Delay` 0.2)
  (goto _label))

(event `GoToTarget`
  (bind _projectilemovementcomponent (`self.ProjectileMovementComponent`))
  (bind _target (`self.FindEnemy`))
  (set `ProjectileMovementComponent.HomingTargetComponent` _target _projectilemovementcomponent)
  (set `ProjectileMovementComponent.bIsHomingProjectile` true _projectilemovementcomponent))

(fn `FindEnemy`
  (returns (Target :type "SceneComponent Object Reference"))
  (bind _homing_target (`self.Homing Target`))
  (bind _outactors (`GameplayStatics.GetAllActorsOfClass` "/Script/GeometryHell2.BaseEnemy"))
  (for _array_element _outactors
    (bind _returnvalue (`KismetMathLibrary.VSize` (- (`self.K2_GetActorLocation` _array_element) (`self.K2_GetActorLocation`))))
    (if (< _returnvalue (`self.ClosestDistance`))
      (set `self.Homing Target` _array_element)
      (set `self.ClosestDistance` _returnvalue)))
  (`/Engine/EditorBlueprintResources/StandardMacros.IsValid` _homing_target
    (:`Is Valid`
      (return (`self.GetComponentByClass` _homing_target "/Script/Engine.SceneComponent")))))

(fn `UserConstructionScript`)