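; BP_SniperRifleWeapon is the sniper rifle weapon Blueprint, which sets its stats from saved player data.
; On BeginPlay it gets the save slot from BP_MainGameInstance and, if a save exists, loads BP_PlayerData to copy sniper damage, fire rate and homing power.
; Without a save the existing values remain, as the nodes that create and write a new save are never run.
; No firing logic is defined in this graph.
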(event `self.ReceiveBeginPlay`
  (bind _asbp_main_game_instance (cast `/Game/MainContent/Logic/BP_MainGameInstance` (`GameplayStatics.GetGameInstance`)))
  (set `self.MainGameInstance` _asbp_main_game_instance)
  (bind _returnvalue (`GameplayStatics.DoesSaveGameExist` (`/Game/MainContent/Logic/BP_MainGameInstance.SaveSlot` (`self.MainGameInstance`))))
  (if _returnvalue
    (bind _returnvalue_2 (`GameplayStatics.LoadGameFromSlot` (`/Game/MainContent/Logic/BP_MainGameInstance.SaveSlot` (`self.MainGameInstance`))))
    (bind _asbp_player_data (cast `/Game/MainContent/Logic/Saves/BP_PlayerData` _returnvalue_2))
    (bind _weaponsdata (`/Game/MainContent/Logic/Saves/BP_PlayerData.WeaponsData` _asbp_player_data))
    (set `self.ProjectileDamage` (break `/Game/MainContent/Logic/Saves/WeaponData/SBP_SniperRifleData` (`.SniperRifle_31_C89204DC45FF6DBA4D2D66ACB783D15E` (break `/Game/MainContent/Logic/Saves/WeaponData/SBP_WeaponsData` _weaponsdata))))
    (set `self.FireRate` (`.SniperRifleFireRate_22_1E7D508D42BFEBEE2BB83EB8E0600F6F` (break `/Game/MainContent/Logic/Saves/WeaponData/SBP_SniperRifleData` (`.SniperRifle_31_C89204DC45FF6DBA4D2D66ACB783D15E` (break `/Game/MainContent/Logic/Saves/WeaponData/SBP_WeaponsData` _weaponsdata)))))
    (set `self.HomingPower` (`.SniperRifleHomingPower_24_692C56CB451A92364A453A8740515D63` (break `/Game/MainContent/Logic/Saves/WeaponData/SBP_SniperRifleData` (`.SniperRifle_31_C89204DC45FF6DBA4D2D66ACB783D15E` (break `/Game/MainContent/Logic/Saves/WeaponData/SBP_WeaponsData` _weaponsdata)))))))

(fn `UserConstructionScript`)