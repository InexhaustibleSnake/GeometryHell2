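; BP_WidgetShow is a one-shot trigger volume that pauses the game and shows a UI widget when BP_Emancipator enters its box.
; The overlap event checks for that exact class, then creates a widget from its Class variable and adds it to the viewport.
; It pauses the game, shows the mouse cursor, switches to UI-only input with the mouse locked, then destroys itself.
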(event `self.BoxTrigger.OnComponentBeginOverlap`
  (params (OverlappedComponent :type "PrimitiveComponent Object Reference") (OtherActor :type "Actor Object Reference") (OtherComp :type "PrimitiveComponent Object Reference") (OtherBodyIndex :type Integer) (bFromSweep :type Boolean) (SweepResult :type "HitResult Structure (by ref)"))
  (bind _returnvalue (`GameplayStatics.GetPlayerController` 0))
  (if (== (`GameplayStatics.GetObjectClass` OtherActor) "/Game/MainContent/Player/BP_Emancipator.BP_Emancipator_C")
    (bind _returnvalue_2 (`|CreateWidget` (`self.Class`)))
    (`UserWidget.AddToViewport` _returnvalue_2 0)
    (`GameplayStatics.SetGamePaused` true)
    (set `PlayerController.bShowMouseCursor` true _returnvalue)
    (`WidgetBlueprintLibrary.SetInputMode_UIOnlyEx` _returnvalue null "LockAlways")
    (`self.K2_DestroyActor`)))

(fn `UserConstructionScript`)