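; Player data container in the save logic, holding per-weapon stats, Emancipator stats and a cores count.
; WeaponsData nests Blaster, Shotgun and SniperRifle stats, each with damage, fire rate and one weapon-specific value.
; Each weapon setter rebuilds the whole struct, replacing its own entry and copying the other two.
; Getters unpack each weapon's stats and the Emancipator's health and stamina maximums; Emancipator data and cores have no setters here.
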(fn `GetBlasterData`
  (returns (Damage :type "Float (double-precision)") (FireRate :type "Float (double-precision)") (Accuracy :type "Float (double-precision)"))
  (bind _weaponsdata (`self.WeaponsData`))
  (return (break `/Game/MainContent/Logic/Saves/WeaponData/SBP_BlasterData` (break `/Game/MainContent/Logic/Saves/WeaponData/SBP_WeaponsData` _weaponsdata)) (`.BlasterFireRate_15_1E7D508D42BFEBEE2BB83EB8E0600F6F` (break `/Game/MainContent/Logic/Saves/WeaponData/SBP_BlasterData` (break `/Game/MainContent/Logic/Saves/WeaponData/SBP_WeaponsData` _weaponsdata))) (`.BlasterAccuracy_16_692C56CB451A92364A453A8740515D63` (break `/Game/MainContent/Logic/Saves/WeaponData/SBP_BlasterData` (break `/Game/MainContent/Logic/Saves/WeaponData/SBP_WeaponsData` _weaponsdata)))))

(fn `GetCoresAmount`
  (returns (NewParam :type "Float (double-precision)"))
  (return (`self.CoresAmount`)))

(fn `GetEmancipatorData`
  (returns (MaxAbilityStamina :type "Float (double-precision)") (MaxHealth :type "Float (double-precision)") (MaxStamina :type "Float (double-precision)"))
  (bind (_emancipatordata_maxabilitystamina _emancipatordata_maxhealth _emancipatordata_maxstamina) (break `/Game/MainContent/Logic/Saves/SBP_EmancipatorData` (`self.EmancipatorData`)))
  (return _emancipatordata_maxabilitystamina _emancipatordata_maxhealth _emancipatordata_maxstamina))

(fn `GetShotgunData`
  (returns (Damage :type "Float (double-precision)") (FireRate :type "Float (double-precision)") (NumOfProjectile :type Integer))
  (bind _weaponsdata (`self.WeaponsData`))
  (return (break `/Game/MainContent/Logic/Saves/WeaponData/SBP_ShotgunData` (`.Shotgun_28_0E0FBEBE4F69CD07D4D1E499849162D4` (break `/Game/MainContent/Logic/Saves/WeaponData/SBP_WeaponsData` _weaponsdata))) (`.ShotgunFireRate_19_1E7D508D42BFEBEE2BB83EB8E0600F6F` (break `/Game/MainContent/Logic/Saves/WeaponData/SBP_ShotgunData` (`.Shotgun_28_0E0FBEBE4F69CD07D4D1E499849162D4` (break `/Game/MainContent/Logic/Saves/WeaponData/SBP_WeaponsData` _weaponsdata)))) (`.ShotgunNumOfProjectiles_20_692C56CB451A92364A453A8740515D63` (break `/Game/MainContent/Logic/Saves/WeaponData/SBP_ShotgunData` (`.Shotgun_28_0E0FBEBE4F69CD07D4D1E499849162D4` (break `/Game/MainContent/Logic/Saves/WeaponData/SBP_WeaponsData` _weaponsdata))))))

(fn `GetSniperRifleData`
  (returns (Damage :type "Float (double-precision)") (FireRate :type "Float (double-precision)") (HomingPower :type "Float (double-precision)"))
  (bind _weaponsdata (`self.WeaponsData`))
  (return (break `/Game/MainContent/Logic/Saves/WeaponData/SBP_SniperRifleData` (`.SniperRifle_31_C89204DC45FF6DBA4D2D66ACB783D15E` (break `/Game/MainContent/Logic/Saves/WeaponData/SBP_WeaponsData` _weaponsdata))) (`.SniperRifleFireRate_22_1E7D508D42BFEBEE2BB83EB8E0600F6F` (break `/Game/MainContent/Logic/Saves/WeaponData/SBP_SniperRifleData` (`.SniperRifle_31_C89204DC45FF6DBA4D2D66ACB783D15E` (break `/Game/MainContent/Logic/Saves/WeaponData/SBP_WeaponsData` _weaponsdata)))) (`.SniperRifleHomingPower_24_692C56CB451A92364A453A8740515D63` (break `/Game/MainContent/Logic/Saves/WeaponData/SBP_SniperRifleData` (`.SniperRifle_31_C89204DC45FF6DBA4D2D66ACB783D15E` (break `/Game/MainContent/Logic/Saves/WeaponData/SBP_WeaponsData` _weaponsdata))))))

(fn `SetBlasterData`
  (params (BlasterDamage :type "Float (double-precision)") (BlasterFireRate :type "Float (double-precision)") (BlasterAccuracy :type "Float (double-precision)"))
  (bind (_weaponsdata_blaster _weaponsdata_shotgun _weaponsdata_sniperrifle) (break `/Game/MainContent/Logic/Saves/WeaponData/SBP_WeaponsData` (`self.WeaponsData`)))
  (set `self.WeaponsData` (make `/Game/MainContent/Logic/Saves/WeaponData/SBP_WeaponsData` (make `/Game/MainContent/Logic/Saves/WeaponData/SBP_BlasterData` BlasterDamage BlasterFireRate BlasterAccuracy) _weaponsdata_shotgun _weaponsdata_sniperrifle)))

(fn `SetShotgunData`
  (params (ShotgunDamage :type "Float (double-precision)") (ShotgunFireRate :type "Float (double-precision)") (ShotgunNumOfProjectiles :type Integer))
  (bind (_weaponsdata_blaster _weaponsdata_shotgun _weaponsdata_sniperrifle) (break `/Game/MainContent/Logic/Saves/WeaponData/SBP_WeaponsData` (`self.WeaponsData`)))
  (set `self.WeaponsData` (make `/Game/MainContent/Logic/Saves/WeaponData/SBP_WeaponsData` _weaponsdata_blaster (make `/Game/MainContent/Logic/Saves/WeaponData/SBP_ShotgunData` ShotgunDamage ShotgunFireRate ShotgunNumOfProjectiles) _weaponsdata_sniperrifle)))

(fn `SetSniperRifleData`
  (params (SniperRifleDamage :type "Float (double-precision)") (SniperRifleFireRate :type "Float (double-precision)") (SniperRifleHomingPower :type "Float (double-precision)"))
  (bind (_weaponsdata_blaster _weaponsdata_shotgun) (break `/Game/MainContent/Logic/Saves/WeaponData/SBP_WeaponsData` (`self.WeaponsData`)))
  (set `self.WeaponsData` (make `/Game/MainContent/Logic/Saves/WeaponData/SBP_WeaponsData` _weaponsdata_blaster _weaponsdata_shotgun (make `/Game/MainContent/Logic/Saves/WeaponData/SBP_SniperRifleData` SniperRifleDamage SniperRifleFireRate SniperRifleHomingPower))))