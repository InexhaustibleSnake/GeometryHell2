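; Save object that stores tuning parameters for three weapons: blaster, shotgun and sniper rifle.
; Each weapon has a setter and getter pair that writes or returns its damage, fire rate and one weapon-specific stat.
; That extra stat is accuracy for the blaster, projectile count for the shotgun and homing power for the sniper rifle.
; It only holds data, with no validation or disk save/load logic in these graphs.
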(fn `GetBlasterParams`
  (returns (BlasterDamage :type "Float (double-precision)") (BlasterFireRate :type "Float (double-precision)") (BlasterAccuracy :type "Float (double-precision)"))
  (return (`self.BlasterDamage`) (`self.BlasterFireRate`) (`self.BlasterAccuracy`)))

(fn `GetShotgunParams`
  (returns (ShotgunDamage :type "Float (double-precision)") (ShotgunFireRate :type "Float (double-precision)") (ShotgunNumOfProjectiles :type Integer))
  (return (`self.ShotgunDamage`) (`self.ShotgunFireRate`) (`self.ShotgunNumOfProjectiles`)))

(fn `GetSniperRifleParams`
  (returns (SniperRifleDamage :type "Float (double-precision)") (SniperRifleFireRate :type "Float (double-precision)") (SniperRifleHomingPower :type "Float (double-precision)"))
  (return (`self.SniperRifleDamage`) (`self.SniperRifleFireRate`) (`self.SniperRifleHomingPower`)))

(fn `SetBlasterParams`
  (params (BlasterDamage :type "Float (double-precision)") (BlasterFireRate :type "Float (double-precision)") (BlasterAccuracy :type "Float (double-precision)"))
  (set `self.BlasterDamage` BlasterDamage)
  (set `self.BlasterFireRate` BlasterFireRate)
  (set `self.BlasterAccuracy` BlasterAccuracy))

(fn `SetShotgunParams`
  (params (ShotgunDamage :type "Float (double-precision)") (ShotgunFireRate :type "Float (double-precision)") (ShotgunNumOfProjectiles :type Integer))
  (set `self.ShotgunDamage` ShotgunDamage)
  (set `self.ShotgunFireRate` ShotgunFireRate)
  (set `self.ShotgunNumOfProjectiles` ShotgunNumOfProjectiles))

(fn `SetSniperRifleParams`
  (params (SniperRifleDamage :type "Float (double-precision)") (SniperRifleFireRate :type "Float (double-precision)") (SniperRifleHomingPower :type "Float (double-precision)"))
  (set `self.SniperRifleDamage` SniperRifleDamage)
  (set `self.SniperRifleFireRate` SniperRifleFireRate)
  (set `self.SniperRifleHomingPower` SniperRifleHomingPower))