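; BP_Checkpoint is a one-shot checkpoint actor that saves progress when the player character overlaps it.
; It loads the BP_PlayerData save from the slot named in BP_MainGameInstance, or creates one if none exists.
; It writes its own transform and the current level name into that save, saves it to the slot, then destroys itself.
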(event `self.ReceiveActorBeginOverlap`
  (params (OtherActor :type "Actor Object Reference"))
  (if (== OtherActor (`GameplayStatics.GetPlayerCharacter` 0))
    (bind _asbp_main_game_instance (cast `/Game/MainContent/Logic/BP_MainGameInstance` (`GameplayStatics.GetGameInstance`)))
    (set `self.MainGameInstance` _asbp_main_game_instance)
    (bind _returnvalue (`GameplayStatics.DoesSaveGameExist` (`/Game/MainContent/Logic/BP_MainGameInstance.SaveSlot` (`self.MainGameInstance`))))
    (if _returnvalue
      (bind _returnvalue_2 (`GameplayStatics.LoadGameFromSlot` (`/Game/MainContent/Logic/BP_MainGameInstance.SaveSlot` (`self.MainGameInstance`))))
      (bind _asbp_player_data (cast `/Game/MainContent/Logic/Saves/BP_PlayerData` _returnvalue_2))
      (set `self.SaveData` _asbp_player_data)
      (else
        (bind _returnvalue_3 (`GameplayStatics.CreateSaveGameObject` "/Game/MainContent/Logic/Saves/BP_PlayerData.BP_PlayerData_C"))
        (set `self.SaveData` _returnvalue_3)))
    (bind _returnvalue_4 (`GameplayStatics.GetCurrentLevelName` true))
    (set `/Game/MainContent/Logic/Saves/BP_PlayerData.LevelAndTransformData` (make `/Game/MainContent/Logic/Saves/SBP_LevelAndTransform` (`self.GetTransform`) _returnvalue_4) (`self.SaveData`))
    (`GameplayStatics.SaveGameToSlot` (`self.SaveData`) (`/Game/MainContent/Logic/BP_MainGameInstance.SaveSlot` (`self.MainGameInstance`)))
    (`self.K2_DestroyActor`)))

(fn `UserConstructionScript`)