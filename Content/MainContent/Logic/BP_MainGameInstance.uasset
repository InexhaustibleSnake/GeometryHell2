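; Game instance that restores saved progress, reading the core count from the save on init and binding a load event.
; The load event opens a level, waits briefly, then calls SetPlayerTransform.
; A separate OpenLevel function opens the level named in the save data.
; SetPlayerTransform only loads and casts the save to BP_PlayerData, as its node that moves the player is disconnected.
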(event `self.ReceiveInit`
  (add `self.Load` (delegate `Load_Event`))
  (bind _asbp_player_data (`/Game/MainContent/Logic/BFL_Main.LoadSaveData`))
  (set `self.NumOfCores` (`/Game/MainContent/Logic/Saves/BP_PlayerData.GetCoresAmount` _asbp_player_data)))

(event `Load_Event`
  (`self.OpenLevel`)
  (`KismetSystemLibrary.Delay` 0.2)
  (`self.SetPlayerTransform`))

(fn `OpenLevel`
  (bind _asbp_player_data (`/Game/MainContent/Logic/BFL_Main.LoadSaveData`))
  (bind (_levelandtransformdata_playertransform _levelandtransformdata_levelname) (break `/Game/MainContent/Logic/Saves/SBP_LevelAndTransform` (`/Game/MainContent/Logic/Saves/BP_PlayerData.LevelAndTransformData` _asbp_player_data)))
  (`GameplayStatics.OpenLevel` (`KismetStringLibrary.Conv_StringToName` _levelandtransformdata_levelname)))

(fn `SetPlayerTransform`
  (bind _returnvalue (`GameplayStatics.LoadGameFromSlot` (`self.SaveSlot`)))
  (cast `/Game/MainContent/Logic/Saves/BP_PlayerData` _returnvalue))