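; Game mode for the level select screen, setting up save state and UI when play begins.
; It loads the player save from the game instance's slot, clears the current level data and writes it back.
; It then adds the level select widget to the viewport, switches the player to UI-only input and shows the mouse cursor.
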(event `self.ReceiveBeginPlay`
  (bind _returnvalue (`GameplayStatics.GetPlayerController` 0))
  (bind _asbp_main_game_instance (cast `/Game/MainContent/Logic/BP_MainGameInstance` (`GameplayStatics.GetGameInstance`)))
  (bind _saveslot (`/Game/MainContent/Logic/BP_MainGameInstance.SaveSlot` _asbp_main_game_instance))
  (bind _returnvalue_2 (`GameplayStatics.LoadGameFromSlot` _saveslot))
  (bind _asbp_player_data (cast `/Game/MainContent/Logic/Saves/BP_PlayerData` _returnvalue_2))
  (set `/Game/MainContent/Logic/Saves/BP_PlayerData.CurrentLevelData` (make `/Game/MainContent/Logic/Saves/SBP_CurrentLevelData` 0.0) _asbp_player_data)
  (`GameplayStatics.SaveGameToSlot` _asbp_player_data _saveslot)
  (bind _returnvalue_3 (`|CreateWidget` "/Game/MainContent/UI/WBP_LevelSelect.WBP_LevelSelect_C"))
  (`UserWidget.AddToViewport` _returnvalue_3 0)
  (`WidgetBlueprintLibrary.SetInputMode_UIOnlyEx` _returnvalue null)
  (set `PlayerController.bShowMouseCursor` true _returnvalue))

(fn `UserConstructionScript`)