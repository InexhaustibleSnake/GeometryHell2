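; Interactive spline platform that the player triggers once to set it moving.
; Overlap by the configured class shows an interact widget and enables use; leaving removes the widget but does not clear the usable flag.
; The interact event locks out further use, removes the prompt and plays a timeline at a configurable rate, feeding its track into MovePlatform each update.
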(event `self.ReceiveBeginPlay`)

(event `self.InteractTrigger.OnComponentBeginOverlap`
  (params (OverlappedComponent :type "PrimitiveComponent Object Reference") (OtherActor :type "Actor Object Reference") (OtherComp :type "PrimitiveComponent Object Reference") (OtherBodyIndex :type Integer) (bFromSweep :type Boolean) (SweepResult :type "HitResult Structure (by ref)"))
  (if (and (== (`GameplayStatics.GetObjectClass` OtherActor) (`self.ClassToInteract`)) (not (`self.WasUsed`)))
    (bind _returnvalue (`|CreateWidget` "/Game/MainContent/UI/WBP_Interact.WBP_Interact_C"))
    (bind _output_get (set `self.InteractWidget` _returnvalue))
    (`UserWidget.AddToViewport` _output_get 0)
    (set `self.CanUse` true)))

(event `self.InteractTrigger.OnComponentEndOverlap`
  (params (OverlappedComponent :type "PrimitiveComponent Object Reference") (OtherActor :type "Actor Object Reference") (OtherComp :type "PrimitiveComponent Object Reference") (OtherBodyIndex :type Integer))
  (if (== (`GameplayStatics.GetObjectClass` OtherActor) (`self.ClassToInteract`))
    (`Widget.RemoveFromParent` (`self.InteractWidget`))))

(event `self.Interact.OnInteract`
  (if (and (not (`self.WasUsed`)) (`self.CanUse`))
    (set `self.WasUsed` true)
    (set `self.CanUse` false)
    (`Widget.RemoveFromParent` (`self.InteractWidget`))
    (`TimelineComponent.SetPlayRate` (`self.Timeline_0_0`) (`self.PlayRate`))
    (bind (_direction _newtrack_0) (`Timeline|Timeline_0_0` :!via `PlayFromStart`)
      (:`Update`
        (`self.MovePlatform` _newtrack_0)))))

(fn `UserConstructionScript`)