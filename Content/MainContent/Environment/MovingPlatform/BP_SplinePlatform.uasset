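; Moving platform actor that carries its Platform component along a Spline, driven by a timeline that starts on BeginPlay.
; Each timeline update passes the track value to MovePlatform, which scales it by spline length to get a distance along the path.
; The platform takes the spline's world location and local roll and yaw at that distance, with pitch zeroed and no sweep.
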(event `self.ReceiveBeginPlay`
  (bind (_direction _newtrack_0) (`Timeline|Timeline_0` :!via `PlayFromStart`)
    (:`Update`
      (`self.MovePlatform` _newtrack_0))))

(fn `MovePlatform`
  (params (MoveTime :type "Float (double-precision)"))
  (bind _returnvalue (* MoveTime (`SplineComponent.GetSplineLength` (`self.Spline`))))
  (bind (_returnvalue_roll _returnvalue_pitch _returnvalue_yaw) (`KismetMathLibrary.BreakRotator` (`SplineComponent.GetRotationAtDistanceAlongSpline` (`self.Spline`) _returnvalue "Local")))
  (`SceneComponent.K2_SetWorldLocation` (`self.Platform`) (`SplineComponent.GetLocationAtDistanceAlongSpline` (`self.Spline`) _returnvalue "World") false false)
  (`SceneComponent.K2_SetRelativeRotation` (`self.Platform`) (`KismetMathLibrary.MakeRotator` _returnvalue_roll 0.0 _returnvalue_yaw) false false))

(fn `UserConstructionScript`)