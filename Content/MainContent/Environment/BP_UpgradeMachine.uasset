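; BP_UpgradeMachine is an environment interactable that opens an upgrade menu for the player.
; Its Box overlap shows or removes a prompt widget for the player character and tracks whether the player is in range.
; An OnInteract event bound from Interact at BeginPlay creates WBP_UpgradeMachine when in range, switches to UI-only input with a visible cursor and pauses the game.
; Closing the menu and unpausing are not handled here.
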(event `self.Box.OnComponentBeginOverlap`
  (params (OverlappedComponent :type "PrimitiveComponent Object Reference") (OtherActor :type "Actor Object Reference") (OtherComp :type "PrimitiveComponent Object Reference") (OtherBodyIndex :type Integer) (bFromSweep :type Boolean) (SweepResult :type "HitResult Structure (by ref)"))
  (if (== OtherActor (`GameplayStatics.GetPlayerCharacter` 0))
    (bind _returnvalue (`|CreateWidget` "/Game/MainContent/UI/Upgrade/WBP_OnUpgradeMachineOverlap.WBP_OnUpgradeMachineOverlap_C"))
    (bind _output_get (set `self.WidgetInteract` _returnvalue))
    (`UserWidget.AddToViewport` _output_get 0)
    (set `self.PlayerOverlap` true)))

(event `self.Box.OnComponentEndOverlap`
  (params (OverlappedComponent :type "PrimitiveComponent Object Reference") (OtherActor :type "Actor Object Reference") (OtherComp :type "PrimitiveComponent Object Reference") (OtherBodyIndex :type Integer))
  (if (== OtherActor (`GameplayStatics.GetPlayerCharacter` 0))
    (`Widget.RemoveFromParent` (`self.WidgetInteract`))
    (set `self.PlayerOverlap` false)))

(event `self.ReceiveBeginPlay`
  (add `InteractComponent.OnInteract` (`self.Interact`) (delegate `OnInteract_Event_0`)))

(event `OnInteract_Event_0`
  (bind _returnvalue (`GameplayStatics.GetPlayerController` 0))
  (if (`self.PlayerOverlap`)
    (bind _returnvalue_2 (`|CreateWidget` "/Game/MainContent/UI/Upgrade/WBP_UpgradeMachine.WBP_UpgradeMachine_C"))
    (bind _output_get (set `self.UpgradeWidget` _returnvalue_2))
    (`UserWidget.AddToViewport` _output_get 0)
    (`WidgetBlueprintLibrary.SetInputMode_UIOnlyEx` _returnvalue null "LockAlways")
    (set `PlayerController.bShowMouseCursor` true _returnvalue)
    (`GameplayStatics.SetGamePaused` true)))

(fn `UserConstructionScript`)