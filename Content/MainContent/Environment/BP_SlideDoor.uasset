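; BP_SlideDoor is a door that slides upward for the player only when no enemies are in a fight.
; A box overlap checks the player controller's enemy count, then a timeline lerps the mesh up and reverses after a short delay.
; An overlap during a fight instead teleports the player to the Scene component's location, if an earlier out-of-combat overlap has set WasOpened.
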(event `self.ReceiveBeginPlay`
  (bind _asbp_emancipator (cast `/Game/MainContent/Player/BP_Emancipator` (`GameplayStatics.GetPlayerCharacter` 0)))
  (set `self.Player` _asbp_emancipator)
  (bind _asbp_main_player_controller (cast `/Game/MainContent/Player/BP_MainPlayerController` (`Pawn.GetController` (`self.Player`))))
  (set `self.PlayerController` _asbp_main_player_controller))

(event `self.Box.OnComponentBeginOverlap`
  (params (OverlappedComponent :type "PrimitiveComponent Object Reference") (OtherActor :type "Actor Object Reference") (OtherComp :type "PrimitiveComponent Object Reference") (OtherBodyIndex :type Integer) (bFromSweep :type Boolean) (SweepResult :type "HitResult Structure (by ref)"))
  (if (== (`MainPlayerController.GetEnemiesInFight` (`self.PlayerController`)) 0)
    (set `self.WasOpened` true)
    (if (== OtherActor (`self.Player`))
      (bind (_direction _newtrack_0) (`Timeline|Timeline_0` :!via `PlayFromStart` :!label _label)
        (:`Update`
          (`SceneComponent.K2_SetRelativeLocation` (`self.DoorMesh`) (`KismetMathLibrary.VLerp` (0.0 0.0 0.0) (0.0 0.0 250.0) _newtrack_0) false false))
        (:`Finished`
          (`KismetSystemLibrary.Delay` 2.0)
          (goto _label :!via `Reverse`))))
    (elif (`self.WasOpened`)
      (`self.K2_SetActorLocation` (`self.Player`) (`SceneComponent.K2_GetComponentLocation` (`self.Scene`)) false false))))

(fn `UserConstructionScript`)