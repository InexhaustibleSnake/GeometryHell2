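; Interactive platform actor that travels along a spline when the player interacts with it.
; InteractTrigger shows an interact widget while an overlapping actor of exactly ClassToInteract is inside, and removes it on exit.
; OnInteract removes the prompt and plays a timeline from the start, whose track samples the spline to set the platform's relative location and align its rotation to the spline direction.
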(event `self.InteractTrigger.OnComponentBeginOverlap`
  (params (OverlappedComponent :type "PrimitiveComponent Object Reference") (OtherActor :type "Actor Object Reference") (OtherComp :type "PrimitiveComponent Object Reference") (OtherBodyIndex :type Integer) (bFromSweep :type Boolean) (SweepResult :type "HitResult Structure (by ref)"))
  (if (== (`GameplayStatics.GetObjectClass` OtherActor) (`self.ClassToInteract`))
    (bind _returnvalue (`|CreateWidget` "/Game/MainContent/UI/WBP_Interact.WBP_Interact_C"))
    (bind _output_get (set `self.InteractWidget` _returnvalue))
    (`UserWidget.AddToViewport` _output_get 0)))

(event `self.InteractTrigger.OnComponentEndOverlap`
  (params (OverlappedComponent :type "PrimitiveComponent Object Reference") (OtherActor :type "Actor Object Reference") (OtherComp :type "PrimitiveComponent Object Reference") (OtherBodyIndex :type Integer))
  (if (== (`GameplayStatics.GetObjectClass` OtherActor) (`self.ClassToInteract`))
    (`Widget.RemoveFromParent` (`self.InteractWidget`))))

(event `self.Interact.OnInteract`
  (`Widget.RemoveFromParent` (`self.InteractWidget`))
  (bind (_direction _newtrack_0) (`Timeline|Timeline_0` :!via `PlayFromStart`)
    (:`Update`
      (`SceneComponent.K2_SetRelativeTransform` (`self.Platform`) (`KismetMathLibrary.MakeTransform` (`SplineComponent.GetLocationAtTime` (`self.Spline`) _newtrack_0 "Local" false) (`KismetMathLibrary.Conv_VectorToRotator` (`SplineComponent.GetDirectionAtTime` (`self.Spline`) _newtrack_0 "Local" false)) (`SceneComponent.K2_GetComponentScale` (`self.Platform`))) false false))))

(fn `UserConstructionScript`)